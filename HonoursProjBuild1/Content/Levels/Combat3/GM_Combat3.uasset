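; GM_Combat3, apparently the Combat3 level's game mode, creates the battle interface widget on BeginPlay and handles player input.
; Navigate, Select, Refresh and InitiativeCheck actions call same-named functions defined outside this graph, with one boolean setting navigation direction.
; ToggleVisuals toggles the widget's visibility, and TTSCallout passes the Blueprint to the widget for what appears to be text-to-speech.
; Escape quits the game.
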(event `self.ReceiveBeginPlay`
  (bind _returnvalue (`|CreateWidget` "/Game/UI/WDG_BattleInterface.WDG_BattleInterface_C" (`GameplayStatics.GetPlayerController` 0)))
  (`UserWidget.AddToViewport` _returnvalue 0))

(event `InputAction|ToggleVisuals`
  (params (Key :type "Key Structure"))
  (:`Pressed`
    (`/Game/UI/WDG_BattleInterface.ToggleVisibility` (stale `self.ReceiveBeginPlay` _returnvalue))))

(event `InputAction|NavigateForward`
  (params (Key :type "Key Structure"))
  (:`Pressed`
    (`self.Navigate` false)))

(event `InputAction|TTSCallout`
  (params (Key :type "Key Structure"))
  (:`Pressed`
    (`/Game/UI/WDG_BattleInterface.TTSCallout` (stale `self.ReceiveBeginPlay` _returnvalue) self)))

(event `InputAction|NavigateBackward`
  (params (Key :type "Key Structure"))
  (:`Pressed`
    (`self.Navigate` true)))

(event `InputAction|Select`
  (params (Key :type "Key Structure"))
  (:`Pressed`
    (`self.Select`)))

(event `InputAction|Refresh`
  (params (Key :type "Key Structure"))
  (:`Pressed`
    (`self.Refresh`)))

(event `InputAction|InitiativeCheck`
  (params (Key :type "Key Structure"))
  (:`Pressed`
    (`self.InitiativeCheck`)))

(event `Key|Escape`
  (params (Key :type "Key Structure"))
  (:`Pressed`
    (`KismetSystemLibrary.QuitGame` null "Quit" true)))

(fn `UserConstructionScript`)