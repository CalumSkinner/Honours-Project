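; GM_Base, apparently a game mode, routes player input for a battle game with text-to-speech support.
; On play it creates a hidden battle interface widget, which input can toggle or ask for a TTS callout.
; Other actions call navigation, selection, refresh, initiative and glossary functions defined outside this graph, and Escape quits.
; Selecting in the Glossary state speaks the current entry's description through the text-to-speech subsystem.
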(event `self.ReceiveBeginPlay`
  (bind _returnvalue (`|CreateWidget` "/Game/UI/WDG_BattleInterface.WDG_BattleInterface_C" (`GameplayStatics.GetPlayerController` 0)))
  (`UserWidget.AddToViewport` _returnvalue 0)
  (`Widget.SetVisibility` _returnvalue "Hidden"))

(event `InputAction|ToggleVisuals`
  (params (Key :type "Key Structure"))
  (:`Pressed`
    (`/Game/UI/WDG_BattleInterface.ToggleVisibility` (stale `self.ReceiveBeginPlay` _returnvalue))))

(event `InputAction|NavigateForward`
  (params (Key :type "Key Structure"))
  (:`Pressed`
    (`self.Navigate` false)))

(event `InputAction|TTSCallout`
  (params (Key :type "Key Structure"))
  (:`Pressed`
    (`/Game/UI/WDG_BattleInterface.TTSCallout` (stale `self.ReceiveBeginPlay` _returnvalue) self)))

(event `InputAction|NavigateBackward`
  (params (Key :type "Key Structure"))
  (:`Pressed`
    (`self.Navigate` true)))

(event `InputAction|Select`
  (params (Key :type "Key Structure"))
  (bind _returnvalue (subsystem `TextToSpeechEngineSubsystem`))
  (bind _channel_one (`self.Channel One`))
  (bind (_output_sound _output_description) (break `GlossaryEntry` (`|GetArrayItem` (`self.AudioGlossary`) (`self.Navigator`))))
  (:`Pressed`
    (`self.Select`)
    (switch `EGameState` (`self.State`)
      (:`Glossary`
        (`TextToSpeechEngineSubsystem.AddDefaultChannel` _returnvalue _channel_one)
        (`TextToSpeechEngineSubsystem.ActivateChannel` _returnvalue _channel_one)
        (`TextToSpeechEngineSubsystem.SpeakOnChannel` _returnvalue _channel_one _output_description)))))

(event `InputAction|Refresh`
  (params (Key :type "Key Structure"))
  (:`Pressed`
    (`self.Refresh`)))

(event `InputAction|InitiativeCheck`
  (params (Key :type "Key Structure"))
  (:`Pressed`
    (`self.InitiativeCheck`)))

(event `Key|Escape`
  (params (Key :type "Key Structure"))
  (:`Pressed`
    (`KismetSystemLibrary.QuitGame` null "Quit" true)))

(event `InputAction|CheckGlossary`
  (params (Key :type "Key Structure"))
  (:`Pressed`
    (`self.CheckGlossary`)))

(fn `UserConstructionScript`)