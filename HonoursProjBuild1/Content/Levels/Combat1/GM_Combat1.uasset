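; GM_Combat1 is the Combat1 level's game mode, setting up the battle interface and handling its menu-style inputs.
; On BeginPlay it creates WDG_BattleInterface for the first player controller and adds it to the viewport.
; NavigateForward and NavigateBackward input actions share one Navigate call with a direction flag, while Select and Refresh trigger their namesake calls.
; The logic behind these calls is defined outside these graphs.
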(event `self.ReceiveBeginPlay`
  (bind _returnvalue (`|CreateWidget` "/Game/UI/WDG_BattleInterface.WDG_BattleInterface_C" (`GameplayStatics.GetPlayerController` 0)))
  (`UserWidget.AddToViewport` _returnvalue 0))

(event `InputAction|NavigateForward`
  (params (Key :type "Key Structure"))
  (:`Pressed`
    (`self.Navigate` false)))

(event `InputAction|NavigateBackward`
  (params (Key :type "Key Structure"))
  (:`Pressed`
    (`self.Navigate` true)))

(event `InputAction|Select`
  (params (Key :type "Key Structure"))
  (:`Pressed`
    (`self.Select`)))

(event `InputAction|Refresh`
  (params (Key :type "Key Structure"))
  (:`Pressed`
    (`self.Refresh`)))

(fn `UserConstructionScript`)